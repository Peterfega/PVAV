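; Zombie spawner actor that keeps adding BP_Zombie_Jaku AI pawns at its Billboard's location while fewer than 20 exist in the world.
; Tick calls the Spawn event every frame, which counts all zombies of that class with GetAllActorsOfClass.
; Below the cap, a three-second Delay paces spawning, then a Niagara system and a new zombie spawn together at the Billboard.
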(event Custom|Spawn
  (bind _billboard (Variables|Default|GetBillboard))
  (bind _returnvalue (Transformation|GetWorldLocation _billboard))
  (bind _outactors (Actor|GetAllActorsOfClass "/Game/Zombies/BP_Zombie_Jaku.BP_Zombie_Jaku_C"))
  (if (<= (Utilities|Array|Length _outactors) 19)
    (Utilities|FlowControl|Delay 3.0)
    (Niagara|SpawnSystematLocation 0 _returnvalue)
    (AI|SpawnAIFromClass "/Game/Zombies/BP_Zombie_Jaku.BP_Zombie_Jaku_C" 0 _returnvalue "0, 0, 0" false 0)))

(event EventTick
  (params (DeltaSeconds :type Float%20%28single-precision%29))
  (CallFunction|Spawn))

(fn ConstructionScript)